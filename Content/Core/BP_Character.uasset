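; Texas Hold'em player character that displays five public and two private cards as static meshes and opens the start and wait widgets.
; On the local controller, it binds to PlayerController new-game and end-game delegates, retrying until the cast succeeds, to show face-down cards or the wait screen.
; Card handlers derive rank and suit from CardID, offset a dynamic material to that face and flip the mesh upright.
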(event Custom|SwitchVisible
  (params (bNewVisibility :type Boolean))
  (Rendering|SetVisibility (Variables|Default|GetStaticMesh2) bNewVisibility false))

(event Custom|WaitGamePlay
  (params (RemainChips :type Integer))
  (Utilities|IsValid (Variables|Default|GetWaitWidget)
    (:Is%20Valid
      (UserInterface|Viewport|AddtoViewport (Variables|Default|GetWaitWidget) 0)
      (Variables|/Game/Blueprints/WBP_Wait.WBP_Wait_C|SetPlayerRemainChips (Variables|Default|GetWaitWidget) -1))
    (:Is%20Not%20Valid
      (bind _returnvalue (UserInterface|CreateWidget "/Game/Blueprints/WBP_Wait.WBP_Wait_C" (Game|GetPlayerController 0) RemainChips))
      (bind _output_get (Variables|Default|SetWaitWidget _returnvalue))
      (UserInterface|Viewport|AddtoViewport _output_get 0))))

(event Custom|OnNewGame
  (CallFunction|SwitchVisible true)
  (Transformation|SetRelativeRotation (Variables|Default|GetStaticMesh2) (Variables|Default|GetReverseSide) false false))

(event Custom|OnEndGame
  (CallFunction|WaitGamePlay))

(event EventBeginPlay
  (bind _returnvalue (Game|GetPlayerController 0))
  (bind _returnvalue_2 (Pawn|GetControlRotation _returnvalue :!class /Script/Engine.Controller))
  (|CallParentFunction)
  (CallFunction|SwitchVisible false)
  (if (Class|HoldemCharacter|HoldemIsLocalController)
    (bind _asbp_player_controller (Utilities|Casting|CastToBP_PlayerController (Game|GetPlayerController 0) :!label _label)
      (:then
        (EventDispatchers|BindEventtoOnNewGameDelegate _asbp_player_controller (delegate Custom|OnNewGame))
        (EventDispatchers|BindEventtoOnEndGameDelegate _asbp_player_controller (delegate Custom|OnEndGame))
        (Networking|SwitchHasAuthority
          (:Authority
            (Utilities|FlowControl|Delay 1.0)
            (Pawn|SetControlRotation _returnvalue (Math|Rotator|MakeRotator (.roll _returnvalue_2) (.pitch _returnvalue_2) (.yaw (Transformation|GetActorRotation)))))))
      (:CastFailed
        (Utilities|FlowControl|Delay 0.2)
        (goto _label)))))

(event EventHandleAddPublicCard
  (params (PublicCards :type Array%20of%20Card%20Info%20Structures))
  (Transformation|SetRelativeRotation (Variables|Default|GetStaticMesh0) (Variables|Default|GetReverseSide) false false)
  (for (_array_element _array_index) PublicCards
    (CallFunction|UpdateCardPerformance (.CardID (Utilities|Struct|BreakCardInfo _array_element)) (CallFunction|GetMeshbyIndex _array_index))))

(event EventHandleAddPrivateCard
  (params (PrivateCards :type Array%20of%20Card%20Info%20Structures))
  (Transformation|SetRelativeRotation (Variables|Default|GetStaticMesh5) (Variables|Default|GetReverseSide) false false)
  (for (_array_element _array_index) PrivateCards
    (CallFunction|UpdateCardPerformance (.CardID (Utilities|Struct|BreakCardInfo _array_element)) (CallFunction|GetMeshbyIndex (+ _array_index 5)))))

(event EventOnPlayerStateSet
  (bind _returnvalue (UserInterface|CreateWidget "/Game/Blueprints/WBP_Start.WBP_Start_C" (Game|GetPlayerController 0)))
  (UserInterface|Viewport|AddtoViewport _returnvalue 0))

(fn ConstructionScript
  (Transformation|SetRelativeRotation (Variables|Default|GetStaticMesh0) (Variables|Default|GetReverseSide) false false))

(fn SetCardPicture
  (params (TargetMesh :type Primitive%20Component%20Object%20Reference) (CardNumber :type Integer) (CardType :type Integer))
  (bind _returnvalue (Rendering|Material|CreateDynamicMaterialInstance TargetMesh 1 0 "None" :!class /Script/Engine.PrimitiveComponent))
  (Rendering|Material|SetVectorParameterValue _returnvalue "Translation" (Math|Color|MakeColor (* (Math|Conversions|ToFloat(Integer) CardNumber) 0.996) (Math|Conversions|ToFloat(Integer) CardType) 0.0) :!class /Script/Engine.MaterialInstanceDynamic)
  (Rendering|Material|SetMaterial TargetMesh 1 _returnvalue))

(fn UpdateCardPerformance
  (params (CardID :type Integer) (TargetMesh :type Primitive%20Component%20Object%20Reference))
  (bind _returnvalue (/ CardID 52))
  (bind _returnvalue_2 (* _returnvalue 52))
  (bind _returnvalue_3 (- CardID _returnvalue_2))
  (bind _returnvalue_4 (/ _returnvalue_3 13))
  (CallFunction|SetCardPicture TargetMesh (- _returnvalue_3 (* _returnvalue_4 13)) _returnvalue_4)
  (Transformation|SetRelativeRotation TargetMesh (Variables|Default|GetRightSide) false false))

(fn GetMeshbyIndex
  (params (Index :type Integer))
  (switch int Index
    (:0
      (return (Variables|Default|GetStaticMesh0)))
    (:1
      (return (Variables|Default|GetStaticMesh1)))
    (:2
      (return (Variables|Default|GetStaticMesh2)))
    (:3
      (return (Variables|Default|GetStaticMesh3)))
    (:4
      (return (Variables|Default|GetStaticMesh4)))
    (:5
      (return (Variables|Default|GetStaticMesh5)))
    (:6
      (return (Variables|Default|GetStaticMesh6)))))