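; BP_GameMode is the game mode for a Hold'em card game, seating players at the desk and dealing public cards.
; PostLogin replaces each player's pawn with a possessed BP_Character at the next desk seat and passes that seat to BP_PlayerState, polling with delays until desk and state are valid.
; After a startup delay, BeginPlay adds five unallocated cards to BP_GameState; per-player dealing exists but is unwired.
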(event Custom|SetPlayerLocationInfo
  (params (PlayerController :type Player%20Controller%20Object%20Reference) (InPlayerLocationInfo :type Player%20Location%20Info%20Structure))
  (bind _playerstate (Variables|/Script/Engine.Controller|GetPlayerState PlayerController))
  (Utilities|IsValid _playerstate :!label _label
    (:Is%20Valid
      (bind _asbp_player_state (Utilities|Casting|CastToBP_PlayerState _playerstate))
      (Class|HoldemPlayerState|SetPlayerLocationInfo _asbp_player_state InPlayerLocationInfo))
    (:Is%20Not%20Valid
      (Utilities|FlowControl|Delay 0.2)
      (goto _label))))

(event EventPostLogin
  (params (NewPlayer :type Player%20Controller%20Object%20Reference))
  (bind _returnvalue (Pawn|GetControlledPawn NewPlayer))
  (bind _holdemdesk (Variables|Default|GetHoldemDesk))
  (bind _playernum (Variables|Default|GetPlayerNum))
  (bind _playerslocationinfos (Variables|/Script/Holdem.HoldemDesk|GetPlayersLocationInfos _holdemdesk))
  (bind _output (Utilities|Array|Get(acopy) _playerslocationinfos _playernum))
  (bind _starttransform (Utilities|Struct|BreakPlayerLocationInfo _output))
  (bind (_location _rotation) (Math|Transform|BreakTransform _starttransform))
  (Utilities|IsValid (Variables|Default|GetHoldemDesk) :!label _label
    (:Is%20Valid
      (Utilities|IsValid _returnvalue
        (:Is%20Valid
          (Actor|DestroyActor _returnvalue))
        (:Is%20Not%20Valid
          _))
      (bind _returnvalue_2 (Game|SpawnActorfromClass "/Game/Core/BP_Character.BP_Character_C" (Math|Transform|MakeTransform _location _rotation) "Undefined" NewPlayer 0))
      (Pawn|Possess NewPlayer _returnvalue_2)
      (CallFunction|SetPlayerLocationInfo NewPlayer _output)
      (Math|Integer|IncrementInt (Variables|Default|GetPlayerNum)))
    (:Is%20Not%20Valid
      (Utilities|FlowControl|Delay 0.2)
      (goto _label))))

(event EventBeginPlay
  (Utilities|FlowControl|Delay 5.0)
  (bind _asbp_game_state (Utilities|Casting|CastToBP_GameState (Game|GetGameState)))
  (for _index (range 0 4)
    (Development|PrintString "添加公共卡牌" true true "(R=1.000000,G=1.000000,B=0.000000,A=1.000000)" 2.5)
    (Class|HoldemGameStateBase|AddPublicCard _asbp_game_state (Class|HoldemGameMode|GetUnallocatedCard))))

(fn ConstructionScript)